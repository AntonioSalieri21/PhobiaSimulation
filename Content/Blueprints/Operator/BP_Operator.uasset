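; BP_Operator is an operator actor that lets player controller 1 watch the VR player or switch to a spectator.
; On BeginPlay it caches the first VRPawn; key 2 flip-flops the view target between that pawn and itself.
; Key 1 possesses a BP_Observer, spawned at the operator's transform on first use and then reused.
; Outline highlighting of "Visible"-tagged actors has its timer setup disconnected, and both SetCamera functions are empty stubs.
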(event Custom|VisibilityControl
  (Utilities|FlowControl|Sequence
    (:then_1
      (for _array_element (Variables|Default|GetVisibilityControlActors)
        (if (== (Utilities|Array|Get(acopy) (Variables|/Script/Engine.Actor|GetTags _array_element)) "Visible")
          (Rendering|Material|SetOverlayMaterial (Actor|GetComponentbyClass _array_element "/Script/Engine.MeshComponent") "/Game/Blueprints/UI/Materials/M_Outline_Inst.M_Outline_Inst" :!class /Script/Engine.MeshComponent))))))

(event Custom|ToggleSpectator
  (bind _returnvalue (Game|GetPlayerController 1))
  (Pawn|UnPossess _returnvalue)
  (Utilities|IsValid (Variables|Default|GetSpectator)
    (:Is%20Valid
      (Pawn|Possess _returnvalue (Variables|Default|GetSpectator)))
    (:Is%20Not%20Valid
      (bind _returnvalue_2 (Game|SpawnActorfromClass "/Game/Blueprints/Operator/BP_Observer.BP_Observer_C" (Transformation|GetActorTransform) "Undefined" "MultiplyWithRoot" 0 0))
      (bind _output_get (Variables|Default|SetSpectator _returnvalue_2))
      (Pawn|Possess (Game|GetPlayerController 1) _output_get))))

(event Custom|TogglePlayerView
  (Utilities|FlowControl|FlipFlop
    (:A
      (Game|Player|SetViewTargetwithBlend (Game|GetPlayerController 1) (Variables|Default|GetVR%20Player) 0.0 "VTBlend_Linear" 0.0 false))
    (:B
      (Game|Player|SetViewTargetwithBlend (Game|GetPlayerController 1) self 0.0 "VTBlend_Linear" 0.0 false))))

(event Collision|EventActorBeginOverlap
  (params (OtherActor :type Actor%20Object%20Reference)))

(event EventBeginPlay
  (bind _outactors (Actor|GetAllActorsOfClass "/Game/VRTemplate/Blueprints/VRPawn.VRPawn_C"))
  (Variables|Default|SetVR%20Player (Utilities|Array|Get(acopy) _outactors)))

(event Input|KeyboardEvents|1
  (params (Key :type Key%20Structure :default "None"))
  (:Released
    (CallFunction|ToggleSpectator)))

(event Input|KeyboardEvents|2
  (params (Key :type Key%20Structure :default "None"))
  (:Released
    (CallFunction|TogglePlayerView)))

(fn ConstructionScript)

(fn SetCameratoPlayer)

(fn SetCameratoThreat)