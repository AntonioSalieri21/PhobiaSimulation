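; Player controller that lets an operator switch between a spectator, the VR player's view and the spider enemy.
; Number keys possess a BP_Observer (spawned at BP_SpawnPoint if missing) or the spider via player controller 1, or toggle a view-target switch between the VR pawn and last pawn.
; For operators, a looping timer enables custom depth on VisibilityCheck-tagged actors whose second tag is "Visible", disabling it otherwise.
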(event Custom|VisibilityControl
  (Utilities|FlowControl|Sequence
    (:then_1
      (for _array_element (Variables|Default|GetVisibilityControlActors)
        (if (== (Utilities|Array|Get(acopy) (Variables|/Script/Engine.Actor|GetTags _array_element) 1) "Visible")
          (Rendering|SetRenderCustomDepth (Actor|GetComponentbyClass _array_element "/Script/Engine.MeshComponent") true)
          (Rendering|SetCustomDepthStencilValue (Actor|GetComponentbyClass _array_element "/Script/Engine.MeshComponent") 0)
          (else
            (Rendering|SetRenderCustomDepth (Actor|GetComponentbyClass _array_element "/Script/Engine.MeshComponent") false)))))))

(event Custom|SwitchToSpectator
  (bind _returnvalue (Game|GetPlayerController 1))
  (Pawn|UnPossess _returnvalue)
  (Utilities|IsValid (Variables|Default|GetSpectator)
    (:Is%20Valid
      (Pawn|Possess _returnvalue (Variables|Default|GetSpectator)))
    (:Is%20Not%20Valid
      (bind _returnvalue_2 (Actor|GetActorOfClass "/Game/ASLM/BP_SpawnPoint.BP_SpawnPoint_C"))
      (bind _returnvalue_3 (Game|SpawnActorfromClass "/Game/Blueprints/Operator/BP_Observer.BP_Observer_C" (Transformation|GetActorTransform _returnvalue_2) "Undefined" "MultiplyWithRoot" 0 0))
      (bind _output_get (Variables|Default|SetSpectator _returnvalue_3))
      (Pawn|Possess (Game|GetPlayerController 1) _output_get)))
  (Variables|Default|SetLastPawn (Variables|Default|GetSpectator))
  (Variables|Default|SetIsWatchingPlayer false)
  (Variables|Default|SetIsWatchingEnemy false))

(event Custom|TogglePlayerView
  (if (Variables|Default|GetIsWatchingPlayer)
    (Variables|Default|SetIsWatchingPlayer false)
    (Game|Player|SetViewTargetwithBlend (Variables|Default|GetLastPawn) 0.0 "VTBlend_Linear" 0.0 false)
    (Development|PrintString "To Last Pawn")
    (else
      (Variables|Default|SetIsWatchingPlayer true)
      (Game|Player|SetViewTargetwithBlend (Variables|Default|GetVR%20Player) 0.0 "VTBlend_Linear" 0.0 false)
      (Development|PrintString "To VR")
      (Variables|Default|SetIsWatchingEnemy false))))

(event Custom|ToggleEnemyView
  (bind _returnvalue (Game|GetPlayerController 1))
  (Pawn|UnPossess _returnvalue)
  (Utilities|IsValid (Variables|Default|GetEnemy)
    (:Is%20Valid
      (Pawn|Possess _returnvalue (Variables|Default|GetEnemy))
      (Variables|Default|SetLastPawn (Variables|Default|GetEnemy))
      (Variables|Default|SetIsWatchingPlayer false)
      (Variables|Default|SetIsWatchingEnemy true))))

(event EventBeginPlay
  (bind _outactors (Actor|GetAllActorsOfClass "/Game/VRTemplate/Blueprints/VRPawn.VRPawn_C"))
  (Variables|Default|SetVR%20Player (Utilities|Array|Get(acopy) _outactors))
  (bind _outactors_2 (Actor|GetAllActorsOfClass "/Game/Blueprints/Spider/BP_Spider.BP_Spider_C"))
  (Variables|Default|SetEnemy (Utilities|Array|Get(acopy) _outactors_2))
  (bind _outactors_3 (Actor|GetAllActorswithTag "VisibilityCheck"))
  (Variables|Default|SetVisibilityControlActors _outactors_3)
  (if (Variables|Default|GetIsOperator)
    (Utilities|Time|SetTimerbyEvent (delegate Custom|VisibilityControl) 0.1 true true)))

(event EventTick
  (params (DeltaSeconds :type Float%20%28single-precision%29)))

(event Input|KeyboardEvents|1
  (params (Key :type Key%20Structure :default "None"))
  (:Released
    (CallFunction|SwitchtoSpectator)))

(event Input|KeyboardEvents|2
  (params (Key :type Key%20Structure :default "None"))
  (:Released
    (CallFunction|TogglePlayerView)))

(event Input|KeyboardEvents|3
  (params (Key :type Key%20Structure :default "None"))
  (:Released
    (CallFunction|ToggleEnemyView)))

(fn ConstructionScript)