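; BP_OperatorController is an operator controller that adds the IMC_Operator Enhanced Input mapping context on BeginPlay.
; Its input events for switching to player, spectator and enemy are empty.
; Disconnected logic would possess a spider, possess an observer spawned at a spawn point, or view through the VR pawn.
; Those branches find or spawn their targets when the cached reference is invalid, but none of them runs.
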(event Input|EnhancedActionEvents|EnhancedInputActionIA_SwitchToPlayer
  (params (ActionValue :type Boolean) (ElapsedSeconds :type Float%20%28double-precision%29) (TriggeredSeconds :type Float%20%28double-precision%29) (InputAction :type Input%20Action%20Object%20Reference :default "/Game/Blueprints/Input/IA_SwitchToPlayer.IA_SwitchToPlayer")))

(event Input|EnhancedActionEvents|EnhancedInputActionIA_SwitchToSpectator
  (params (ActionValue :type Boolean) (ElapsedSeconds :type Float%20%28double-precision%29) (TriggeredSeconds :type Float%20%28double-precision%29) (InputAction :type Input%20Action%20Object%20Reference :default "/Game/Blueprints/Input/IA_SwitchToSpectator.IA_SwitchToSpectator")))

(event Input|EnhancedActionEvents|EnhancedInputActionIA_SwitchToEnemy
  (params (ActionValue :type Boolean) (ElapsedSeconds :type Float%20%28double-precision%29) (TriggeredSeconds :type Float%20%28double-precision%29) (InputAction :type Input%20Action%20Object%20Reference :default "/Game/Blueprints/Input/IA_SwitchToEnemy.IA_SwitchToEnemy")))

(event EventBeginPlay
  (Input|AddMappingContext (PlayerController|LocalPlayerSubsystems|GetEnhancedInputLocalPlayerSubsystem self) "/Game/Blueprints/Input/IMC_Operator.IMC_Operator" 0 (Utilities|Struct|MakeModifyContextOptions true false false)))

(event EventTick
  (params (DeltaSeconds :type Float%20%28single-precision%29)))

(fn ConstructionScript)