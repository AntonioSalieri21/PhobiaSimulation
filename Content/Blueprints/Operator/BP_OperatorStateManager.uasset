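; Operator state manager actor that switches the second local player controller (index 1) between spectator, VR player and enemy views.
; BeginPlay caches the first VRPawn and starts in spectator mode, which possesses a BP_Observer spawned at the manager's transform when none exists.
; Player view only changes the view target to the VR pawn, while enemy view possesses the first BP_Spider found.
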(event Custom|SwitchToSpectator
  (Pawn|UnPossess (Game|GetPlayerController 1))
  (Utilities|IsValid (Variables|Default|GetSpectator)
    (:Is%20Valid
      _)
    (:Is%20Not%20Valid
      (bind _returnvalue (Game|SpawnActorfromClass "/Game/Blueprints/Operator/BP_Observer.BP_Observer_C" (Transformation|GetActorTransform) "Undefined" "MultiplyWithRoot" 0 0))
      (bind _output_get (Variables|Default|SetSpectator _returnvalue))))
  (Pawn|Possess (Game|GetPlayerController 1) _output_get))

(event Custom|SwitchToPlayerView
  (Game|Player|SetViewTargetwithBlend (Game|GetPlayerController 1) (Variables|Default|GetVRPlayer) 0.0 "VTBlend_Linear" 0.0 false))

(event Custom|SwitchToEnemyView
  (Pawn|UnPossess (Game|GetPlayerController 1))
  (Utilities|IsValid (Variables|Default|GetSpider)
    (:Is%20Valid
      _)
    (:Is%20Not%20Valid
      (bind _outactors (Actor|GetAllActorsOfClass "/Game/Blueprints/Spider/BP_Spider.BP_Spider_C"))
      (bind _output_get (Variables|Default|SetSpider (Utilities|Array|Get(acopy) _outactors)))))
  (Pawn|Possess (Game|GetPlayerController 1) _output_get))

(event EventBeginPlay
  (Variables|Default|SetOperatorPlayerController (Game|GetPlayerController 1))
  (bind _outactors (Actor|GetAllActorsOfClass "/Game/VRTemplate/Blueprints/VRPawn.VRPawn_C"))
  (Variables|Default|SetVRPlayer (Utilities|Array|Get(acopy) _outactors))
  (CallFunction|SwitchtoSpectator))

(fn ConstructionScript)