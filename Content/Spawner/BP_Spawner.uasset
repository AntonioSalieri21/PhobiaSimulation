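; Spawner actor that keeps up to MaxCount actors of ActorType on surrounding surfaces within a radius.
; Each interval tick it traces a random direction for a hit point clear of nearby pawns.
; Two offset traces around that point derive a surface-aligned rotation, and the actor spawns raised along its up vector.
; Spawns get an optional lifespan, a follow target and activation; their destruction decrements the count.
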(event Custom|PawnDestroyed
  (params (DestroyedPawn :type Actor%20Object%20Reference))
  (Math|Integer|DecrementInt (Variables|Default|GetcurrentCount)))

(event EventBeginPlay)

(event Collision|EventActorBeginOverlap
  (params (OtherActor :type Actor%20Object%20Reference)))

(event EventTick
  (params (DeltaSeconds :type Float%20%28single-precision%29))
  (if (< (Variables|Default|GetcurrentCount) (Variables|Default|GetmaxCount))
    (bind (_spawnlocation _succes) (CallFunction|FindSpawnLocation))
    (if _succes
      (bind (_succes_2 _rotation) (CallFunction|FindRotationforLocation _spawnlocation))
      (if _succes_2
        (CallFunction|SpawnActor _spawnlocation _rotation)))))

(fn ConstructionScript
  (Components|Sphere|SetSphereRadius (Variables|Default|GetSpawn%20Area) (Variables|Default|GetRadius) true)
  (Actor|Tick|SetActorTickInterval (Variables|Default|GetSpawnInterval)))

(fn FindSpawnLocation
  (bind _returnvalue (Transformation|GetActorLocation))
  (bind (_outhit _returnvalue_2) (Class|KismetSystemLibrary|LineTraceSinglebyProfile _returnvalue (+ _returnvalue (* (Math|Random|RandomUnitVector) (Variables|Default|GetRadius))) "IgnoreOnlyPawn" false 0 "None" true))
  (if _returnvalue_2
    (bind _returnvalue_3 (Collision|SphereOverlapActors (.Location (Collision|BreakHitResult _outhit)) (Variables|Default|GetminSpawnDistanceFromPawn) (Utilities|Array|MakeArray "ObjectTypeQuery3") 0))
    (if _returnvalue_3
      (return "0, 0, 0" false)
      (else
        (return (.Location (Collision|BreakHitResult _outhit)) true)))
    (else
      (return "0, 0, 0" false))))

(fn FindRotationforLocation
  (params (location :type Vector))
  (bind _returnvalue (Transformation|GetActorLocation))
  (bind _returnvalue_2 (Transformation|GetActorLocation))
  (LocalVariables|SetSpawnDirection (Math|Vector|GetUnitDirection(Vector) (Transformation|GetActorLocation) location))
  (LocalVariables|SetDirection1 (Math|Vector|GetUnitDirection(Vector) (Transformation|GetActorLocation) (+ location (* (.Y (Math|Rotator|BreakRotIntoAxes (Math|Rotator|MakeRotfromX (LocalVariables|GetSpawnDirection)))) (Variables|Default|GetrotationTestDistance)))))
  (LocalVariables|SetDirection2 (Math|Vector|GetUnitDirection(Vector) (Transformation|GetActorLocation) (+ location (* (.Z (Math|Rotator|BreakRotIntoAxes (Math|Rotator|MakeRotfromX (LocalVariables|GetSpawnDirection)))) (Variables|Default|GetrotationTestDistance)))))
  (bind (_outhit _returnvalue_3) (Class|KismetSystemLibrary|LineTraceSinglebyProfile _returnvalue_2 (+ _returnvalue_2 (* (LocalVariables|GetDirection1) (Variables|Default|GetRadius))) "IgnoreOnlyPawn" false 0 "None" true))
  (if _returnvalue_3
    (LocalVariables|SetRight (Math|Vector|GetUnitDirection(Vector) location (.Location (Collision|BreakHitResult _outhit))))
    (bind (_outhit_2 _returnvalue_4) (Class|KismetSystemLibrary|LineTraceSinglebyProfile _returnvalue (+ _returnvalue (* (LocalVariables|GetDirection2) (Variables|Default|GetRadius))) "IgnoreOnlyPawn" false 0 "None" true))
    (if _returnvalue_4
      (LocalVariables|SetForward (Math|Vector|GetUnitDirection(Vector) location (.Location (Collision|BreakHitResult _outhit_2))))
      (return true (Math|Rotator|MakeRotfromXY (LocalVariables|GetForward) (LocalVariables|GetRight)))
      (else
        (return false "0, 0, 0")))
    (else
      (return false "0, 0, 0"))))

(fn SpawnActor
  (params (spawnLocation :type Vector) (spawnRotation :type Rotator))
  (bind _target (Variables|Default|GetTarget))
  (bind _returnvalue (Game|SpawnActorfromClass (Variables|Default|GetActorType) (Math|Transform|MakeTransform (+ spawnLocation (* (Math|Vector|GetUpVector spawnRotation) (Variables|Default|GetspawnHeight))) spawnRotation) "AlwaysSpawn" "MultiplyWithRoot" 0 0))
  (Math|Integer|IncrementInt (Variables|Default|GetcurrentCount)
    (:%20%20
      (if (!= (Variables|Default|GetlifeSpanSeconds) 0.0)
        (Actor|SetLifeSpan _returnvalue (Variables|Default|GetlifeSpanSeconds)))
      (Game|BindEventtoOnDestroyed _returnvalue (EventDispatchers|CreateEvent :!event Custom|PawnDestroyed))
      (bind _asblack_widow_pawn (Utilities|Casting|CastTo _returnvalue)
        (:then
          (Variables|Default|SetfollowActor _asblack_widow_pawn _target)
          (CallFunction|Activate _asblack_widow_pawn))
        (:CastFailed
          (bind _ascrawler_pawn_base (Utilities|Casting|CastTo _returnvalue))
          (Variables|Default|SetFollowActor _ascrawler_pawn_base _target)
          (CallFunction|EventActivatePawn _ascrawler_pawn_base))))))