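; Game mode for an asymmetric two-player session, pairing a VR player with an operator.
; On PostLogin it gathers the spawn points, spawns a replicated VRPawn or BP_Operator by join index at the matching array entry, then possesses it.
; When the second player joins, the operator receives a reference to the VR pawn.
; SpawnPawns, a local-player alternative matching spawn points by tag, is never run.
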(event EventBeginPlay)

(event EventTick
  (params (DeltaSeconds :type Float%20%28single-precision%29)))

(event EventPostLogin
  (params (NewPlayer :type Player%20Controller%20Object%20Reference))
  (CallFunction|GetPlayerStartPoints)
  (bind _returnvalue (Game|SpawnActorfromClass (Utilities|Select :Index (Variables|Default|GetIndex) :Option%200 "/Game/VRTemplate/Blueprints/VRPawn.VRPawn_C" :Option%201 "/Game/Blueprints/Operator/BP_Operator.BP_Operator_C") (Transformation|GetActorTransform (Utilities|Array|Get(acopy) (Variables|Default|GetPlayerStartArray) (Variables|Default|GetIndex))) "Undefined" "MultiplyWithRoot" NewPlayer 0))
  (Networking|SetReplicates _returnvalue true)
  (bind _aspawn (Utilities|Casting|CastToPawn _returnvalue))
  (Utilities|Array|Add (Variables|Default|GetPlayers) _aspawn)
  (bind _result (Math|Integer|IncrementInt (Variables|Default|GetIndex))
    (:%20%20
      (if (== _result 2)
        (bind _asbp_operator (Utilities|Casting|CastToBP_Operator _returnvalue))
        (bind _asvrpawn (Utilities|Casting|CastToVRPawn (Utilities|Array|Get(acopy) (Variables|Default|GetPlayers))))
        (Variables|/Game/Blueprints/Operator/BP_Operator.BP_Operator_C|SetVR%20Player _asbp_operator _asvrpawn))
      (Pawn|Possess NewPlayer _aspawn))))

(fn ConstructionScript)

(fn GetPlayerStartPoints
  (bind _outactors (Actor|GetAllActorsOfClass "/Game/ASLM/BP_SpawnPoint.BP_SpawnPoint_C"))
  (Variables|Default|SetPlayerStartArray _outactors))

(fn SpawnPawns
  (for _index (range 0 1)
    (Variables|Default|SetIndex _index)
    (for _array_element (Variables|Default|GetPlayerStartArray)
      (Development|PrintString (Variables|/Game/ASLM/BP_SpawnPoint.BP_SpawnPoint_C|GetPlayerTag _array_element))
      (if (== (Variables|/Game/ASLM/BP_SpawnPoint.BP_SpawnPoint_C|GetPlayerTag _array_element) (Utilities|String|ToString(Integer) (Variables|Default|GetIndex)))
        (Class|GameplayStatics|CreatePlayer -1)
        (bind _returnvalue (Game|SpawnActorfromClass (Utilities|Select :Index (Variables|Default|GetIndex) :Option%200 "/Game/VRTemplate/Blueprints/VRPawn.VRPawn_C" :Option%201 "/Game/FirstPerson/Blueprints/BP_FirstPersonCharacter.BP_FirstPersonCharacter_C") (Transformation|GetActorTransform _array_element) "AlwaysSpawn" "MultiplyWithRoot" 0 0))
        (bind _aspawn (Utilities|Casting|CastToPawn _returnvalue)
          (:then
            (Pawn|Possess (Game|GetPlayerController (Variables|Default|GetIndex)) _aspawn))
          (:CastFailed
            (Development|PrintString "Cast failed")))))))

(fn SetCameratoSpectator)